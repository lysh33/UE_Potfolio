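; BP_Switch is a toggle switch actor that activates or releases a list of linked items when something overlaps its trigger.
; Each overlap flips IsPushed, sets a scalar parameter on a dynamic material created in the construction script, and sends the switch or released message to every entry in Items.
; Leftover, unconnected nodes for opening a door and toggling an arrow box's firing never run.
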(event `self.Trigger.OnComponentBeginOverlap`
  (params (OverlappedComponent :type "PrimitiveComponent Object Reference") (OtherActor :type "Actor Object Reference") (OtherComp :type "PrimitiveComponent Object Reference") (OtherBodyIndex :type Integer) (bFromSweep :type Boolean) (SweepResult :type "HitResult Structure (by ref)"))
  (if (`self.Is_Pushed?`)
    (`MaterialInstanceDynamic.SetScalarParameterValue` (`self.Material`) "active_parameter_1" 0.0)
    (set `self.Is_Pushed?` false)
    (for _array_element (`self.Items`)
      (message `/Game/BluePrints/BPI_Item.OnRelesed` _array_element))
    (else
      (`MaterialInstanceDynamic.SetScalarParameterValue` (`self.Material`) "active_parameter_1" 1.0)
      (set `self.Is_Pushed?` true)
      (for _array_element_2 (`self.Items`)
        (message `/Game/BluePrints/BPI_Item.Onswitch` _array_element_2)))))

(fn `UserConstructionScript`
  (bind _returnvalue (`PrimitiveComponent.CreateDynamicMaterialInstance` (`self.StaticMesh`) 0 null))
  (set `self.Material` _returnvalue))